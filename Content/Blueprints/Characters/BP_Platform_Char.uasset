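; BP_Platform_Char is a 2D sprite-based platformer character that defines a shared defeat sequence.
; Defeat runs once behind a flag, disabling capsule collision and releasing the movement plane constraint.
; It then launches the character up and along the right vector using tunable strengths, jumps the Locomotion animation state machine to its defeat node and raises sprite sort priority.
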(event `Defeat`
  (if (not (`self.isDeafeated`))
    (set `self.isDeafeated` true)
    (`PrimitiveComponent.SetCollisionEnabled` (`self.CapsuleComponent`) "NoCollision")
    (`MovementComponent.SetPlaneConstraintEnabled` (`self.CharacterMovement`) false)
    (`self.LaunchOnDefeat`)
    (`PaperZDAnimInstance.JumpToNode` (`self.GetAnimInstance`) "Jump_Defeat" "Locomotion")
    (`PrimitiveComponent.SetTranslucentSortPriority` (`self.Sprite`) 100)))

(fn `LaunchOnDefeat`
  (`self.LaunchCharacter` (+ (* (`KismetMathLibrary.Vector_Up`) (`self.DefeatUpLauncher`)) (* (`KismetMathLibrary.Vector_Right`) (`self.DefeatForwardLauncher`))) true true))

(fn `UserConstructionScript`)